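; BP_Hex is a clickable hex map tile with a randomized terrain type, a barrier or prop mesh, and an access flag.
; The construction script picks the type with a bias toward accessible grass, setting mesh, ground material, scale and Access.
; Clicks on the actor or barrier call OnClick.
; InPathChanged swaps materials for path, enemy-next and clicked states, hiding the barrier on path tiles and restoring the saved terrain material otherwise.
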(event `self.MeshBarrier.OnClicked`
  (params (TouchedComponent :type "PrimitiveComponent Object Reference") (ButtonPressed :type "Key Structure"))
  (`self.onClick` :!label _label))

(event `self.ReceiveActorOnClicked`
  (params (ButtonPressed :type "Key Structure"))
  (goto _label))

(event `self.ReceiveTick`
  (params (DeltaSeconds :type "Float (single-precision)")))

(event `self.InPathChanged`
  (bind _returnvalue (`self.IsInPath`))
  (switch `EIsInPath` _returnvalue
    (:`Empty`
      (`SceneComponent.SetVisibility` (`self.MeshBarrier`) true false)
      (`PrimitiveComponent.SetMaterial` (`self.Mesh`) 2 (`self.PrevMaterial`)))
    (:`InPath`
      (`SceneComponent.SetVisibility` (`self.MeshBarrier`) false false)
      (`PrimitiveComponent.SetMaterial` (`self.Mesh`) 2 "/Game/MyContent/MyMaterials/M_Trigger.M_Trigger"))
    (:`EnemyNext`
      (`SceneComponent.SetVisibility` (`self.MeshBarrier`) false false)
      (`PrimitiveComponent.SetMaterial` (`self.Mesh`) 2 "/Game/MyContent/MyMaterials/M_Trigger_2.M_Trigger_2")))
  (if (`self.m_onClicked`)
    (`PrimitiveComponent.SetMaterial` (`self.Mesh`) 0 "/Game/MyContent/MyMaterials/M_Trigger.M_Trigger")
    (else
      (`PrimitiveComponent.SetMaterial` (`self.Mesh`) 0 "/Engine/EditorMeshes/ColorCalibrator/M_ClearCoatBlack.M_ClearCoatBlack"))))

(fn `UserConstructionScript`
  (bind _returnvalue (`KismetMathLibrary.RandomIntegerInRange` 0 4))
  (bind _returnvalue_2 (`KismetMathLibrary.MakeRandomStream` 0))
  (`KismetMathLibrary.SeedRandomStream` _returnvalue_2)
  (set `self.HexTypeIdx` _returnvalue)
  (if (<= _returnvalue 2)
    (if (not (`KismetMathLibrary.RandomBoolWithWeightFromStream` 0.05 _returnvalue_2))
      (set `self.HexTypeIdx` 3)))
  (switch `int` (`self.HexTypeIdx`)
    (:`Default`
      (`StaticMeshComponent.SetStaticMesh` (`self.MeshBarrier`) "/Game/MyContent/Meshes/HexMap/SM_Barrier_6.SM_Barrier_6" :!label _label)
      (`PrimitiveComponent.SetMaterial` (`self.Mesh`) 2 "/Game/MyContent/MyMaterials/M_Ground_Grass_2.M_Ground_Grass_2")
      (set `self.Scale` (0.1 0.1 0.05))
      (set `self.access` true))
    (:`0`
      (`StaticMeshComponent.SetStaticMesh` (`self.MeshBarrier`) "/Game/MyContent/Meshes/Village/SM_Tree_Var03.SM_Tree_Var03")
      (`PrimitiveComponent.SetMaterial` (`self.Mesh`) 2 "/Game/MyContent/Landscape/M_Landscape.M_Landscape")
      (set `self.Scale` (0.04 0.04 0.04))
      (set `self.access` false :!label _label_2))
    (:`1`
      (`StaticMeshComponent.SetStaticMesh` (`self.MeshBarrier`) "/Game/MyContent/Meshes/HexMap/SM_Barrier_1.SM_Barrier_1")
      (`PrimitiveComponent.SetMaterial` (`self.Mesh`) 2 "/Game/StarterContent/Materials/M_Ground_Grass.M_Ground_Grass")
      (set `self.Scale` (0.04 0.04 0.04))
      (goto _label_2))
    (:`2`
      (`StaticMeshComponent.SetStaticMesh` (`self.MeshBarrier`) "/Game/MyContent/Meshes/HexMap/SM_Barrier_2.SM_Barrier_2")
      (`PrimitiveComponent.SetMaterial` (`self.Mesh`) 2 "/Game/MyContent/MyMaterials/desert_terrain.desert_terrain")
      (set `self.Scale` (0.05 0.05 0.05))
      (goto _label_2))
    (:`3`
      (goto _label)))
  (`SceneComponent.K2_SetWorldTransform` (`self.MeshBarrier`) (`SceneComponent.K2_GetComponentToWorld` (`self.Mesh`)) false true)
  (`SceneComponent.SetRelativeScale3D` (`self.MeshBarrier`) (`self.Scale`))
  (set `self.PrevMaterial` (`PrimitiveComponent.GetMaterial` (`self.Mesh`) 2)))