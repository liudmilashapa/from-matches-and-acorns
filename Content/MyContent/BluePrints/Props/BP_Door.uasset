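; BP_Door is a door prop with fire, steam and sound effects that are removed when it opens.
; The OpenDoor event destroys the fire and steam components and the fire sound, then plays a timeline from the start.
; The timeline drives the door mesh's absolute world yaw, with pitch and roll held at zero, and disables the mesh's collision when finished.
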(event `OpenDoor`
  (`ActorComponent.K2_DestroyComponent` (`self.P_Fire`))
  (`ActorComponent.K2_DestroyComponent` (`self.P_Steam_Lit`))
  (`ActorComponent.K2_DestroyComponent` (`self.Fire_sound`))
  (bind (_direction _rotetionz) (`Timeline|DoorOpenTimeline` :!via `PlayFromStart`)
    (:`Update`
      (`SceneComponent.K2_SetWorldRotation` (`self.SM_Door`) (`KismetMathLibrary.MakeRotator` 0.0 0.0 _rotetionz) false false))
    (:`Finished`
      (`PrimitiveComponent.SetCollisionEnabled` (`self.SM_Door`) "NoCollision"))))

(fn `UserConstructionScript`)