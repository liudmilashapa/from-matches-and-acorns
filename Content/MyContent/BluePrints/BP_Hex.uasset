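; BP_Hex is a hex tile actor that responds to mouse clicks and shows whether it lies on a path.
; Clicks call OnClick, and Tick polls IsInPath to swap one mesh material slot between heatmap and flipbook materials; both functions are defined outside this file.
; Cursor hover sets an alpha brush material on the same slot, which Tick overwrites whenever it runs.
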(event `self.ReceiveActorOnClicked`
  (params (ButtonPressed :type "Key Structure"))
  (`self.onClick`))

(event `self.ReceiveTick`
  (params (DeltaSeconds :type "Float (single-precision)"))
  (bind _returnvalue (`self.IsInPath`))
  (if _returnvalue
    (`PrimitiveComponent.SetMaterial` (`self.Mesh`) 2 "/Engine/EngineDebugMaterials/HeatmapMaterial.HeatmapMaterial")
    (else
      (`PrimitiveComponent.SetMaterial` (`self.Mesh`) 2 "/Engine/ArtTools/RenderToTexture/Materials/Debug/M_TestFlipbookAnimation.M_TestFlipbookAnimation"))))

(event `self.ReceiveActorEndCursorOver`)

(event `self.ReceiveActorBeginCursorOver`
  (`PrimitiveComponent.SetMaterial` (`self.Mesh`) 2 "/Engine/EditorLandscapeResources/AlphaBrushMaterial.AlphaBrushMaterial"))

(fn `UserConstructionScript`)